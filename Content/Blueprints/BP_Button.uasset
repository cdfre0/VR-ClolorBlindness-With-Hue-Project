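; BP_Button is a pressure button that sinks while any actor overlaps its Box and rises back when clear.
; Tick nudges MovablePart in clamped steps between zero and ButtonOffSet, the rest height set in the construction script.
; Reaching the bottom plays a 2D cue and sets IsClicked, with WasClicked blocking repeats until full release.
; A separate GoalToButton overlap only prints the names of static mesh actors.
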(event OnComponentBeginOverlap(GoalToButton)
  (params (OverlappedComponent :type Primitive%20Component%20Object%20Reference) (OtherActor :type Actor%20Object%20Reference) (OtherComp :type Primitive%20Component%20Object%20Reference) (OtherBodyIndex :type Integer) (bFromSweep :type Boolean) (SweepResult :type Hit%20Result%20Structure%20%28by%20ref%29))
  (bind _asstatic_mesh_actor (Utilities|Casting|CastToStaticMeshActor OtherActor))
  (Development|PrintString (Utilities|GetDisplayName _asstatic_mesh_actor)))

(event EventBeginPlay
  (bind _output_get (Variables|Default|SetAudio "/Game/SFX/Random_Cue.Random_Cue")))

(event EventTick
  (params (DeltaSeconds :type Float%20%28single-precision%29))
  (bind _movable_part (Variables|Default|GetMovable%20Part))
  (bind _movable_part_2 (Variables|Default|GetMovable%20Part))
  (bind _relativelocation (Variables|/Script/Engine.SceneComponent|GetRelativeLocation _movable_part_2))
  ;[1 0.3222 0.352] Set Audio
  ;;[1 1 1] Check if Button is pressed fully
  (if (== (.z _relativelocation) 0.0)
    ;[1 1 1] Check if Button was pressed in this iteration
    (if (Variables|Default|GetwasClicked)
      _
      (else
        (Audio|PlaySound2D (stale EventBeginPlay _output_get) 1.0 1.0 0.0 0 0)
        ;[1 1 1] Set variables to new one since It is first press in iteration
        (Variables|Default|SetisClicked true)
        (Variables|Default|SetwasClicked true)))
    (else
      ;[1 1 1] Check if Button came back to normal state to fully start new iteration
      (if (== (.z _relativelocation) (Variables|Default|GetButtonOffSet))
        (Variables|Default|SetwasClicked false))))
  ;[1 1 1] Check if something overlaps button
  (if (> (Utilities|Array|Length (Collision|GetOverlappingActors (Variables|Default|GetBox) 0 :!class /Script/Engine.PrimitiveComponent)) 0)
    (Components|MoveComponentTo _movable_part (Math|Vector|MakeVector 0.0 0.0 (Math|Float|Clamp(Float) (- (.z (Variables|/Script/Engine.SceneComponent|GetRelativeLocation _movable_part)) 3.0) 0.0 (Variables|Default|GetButtonOffSet))) "0, 0, 0" false false 0.001 false)
    (else
      (Components|MoveComponentTo _movable_part (Math|Vector|MakeVector 0.0 0.0 (Math|Float|Clamp(Float) (+ (.z (Variables|/Script/Engine.SceneComponent|GetRelativeLocation _movable_part)) 3.0) 0.0 (Variables|Default|GetButtonOffSet))) "0, 0, 0" false false 0.001 false))))

(fn ConstructionScript
  (bind _buttonoffset (Variables|Default|GetButtonOffSet))
  (Variables|/Script/Engine.ArrowComponent|SetArrowLength (Variables|Default|GetArrow) _buttonoffset)
  (Transformation|SetRelativeLocation (Variables|Default|GetMovable%20Part) (Math|Vector|MakeVector 0.0 0.0 _buttonoffset) false false))