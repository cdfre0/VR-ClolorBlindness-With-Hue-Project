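; BP_Box is a sorting box that scores a Grabbable_SmallCube placed inside it by comparing the cube's ColorValue with its own.
; On BeginPlay it takes one character of its display name as both its text label and its ColorValue, so the actor's name configures it.
; Overlap turns the diode green and gives full Score for a match, partial for exactly one above, minimal otherwise.
; End overlap turns it red and clears Score.
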(event OnComponentBeginOverlap(Box)
  (params (OverlappedComponent :type Primitive%20Component%20Object%20Reference) (OtherActor :type Actor%20Object%20Reference) (OtherComp :type Primitive%20Component%20Object%20Reference) (OtherBodyIndex :type Integer) (bFromSweep :type Boolean) (SweepResult :type Hit%20Result%20Structure%20%28by%20ref%29))
  (bind _colorvalue (Variables|Default|GetColorValue))
  (bind _asgrabbable_small_cube (Utilities|Casting|CastToGrabbable_SmallCube OtherActor))
  (Rendering|Material|SetMaterial (Variables|Default|GetDiode) 0 "/Engine/EngineDebugMaterials/VertexColorViewMode_GreenOnly.VertexColorViewMode_GreenOnly")
  (if (== (Variables|/Game/VRTemplate/Blueprints/Grabbable_SmallCube.Grabbable_SmallCube_C|GetColorValue _asgrabbable_small_cube) _colorvalue)
    (Variables|Default|SetScore 100)
    (elif (== (- (Variables|/Game/VRTemplate/Blueprints/Grabbable_SmallCube.Grabbable_SmallCube_C|GetColorValue _asgrabbable_small_cube) _colorvalue) 1)
      (Variables|Default|SetScore 60)
      (else
        (Variables|Default|SetScore 1)))))

(event OnComponentEndOverlap(Box)
  (params (OverlappedComponent :type Primitive%20Component%20Object%20Reference) (OtherActor :type Actor%20Object%20Reference) (OtherComp :type Primitive%20Component%20Object%20Reference) (OtherBodyIndex :type Integer))
  (Utilities|Casting|CastToGrabbable_SmallCube OtherActor)
  (Rendering|Material|SetMaterial (Variables|Default|GetDiode) 0 "/Engine/EngineDebugMaterials/VertexColorViewMode_RedOnly.VertexColorViewMode_RedOnly")
  (Variables|Default|SetScore 0))

(event EventBeginPlay
  (bind _self self)
  (bind _returnvalue (Utilities|GetDisplayName _self))
  (bind _returnvalue_2 (Utilities|String|GetSubstring _returnvalue 7))
  (Rendering|Components|TextRender|SetText (Variables|Default|GetTextRender) (Utilities|Text|ToText(String) _returnvalue_2))
  (Variables|Default|SetColorValue (Math|Conversions|ToInteger(Byte) _returnvalue_2)))

(fn ConstructionScript)